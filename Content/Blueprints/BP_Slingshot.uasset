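; Pinball slingshot bumper that kicks the ball away and awards points when hit.
; On overlap it plays an attached sound, then for a bp_ball adds score through PinballGameMode and applies a velocity-change impulse opposite the capsule's forward vector.
; A timeline then drives the PercentOut scalar on the mesh materials, animating the band bounce through a dynamic M_MorphBand instance created in the construction script.
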(event `self.ReceiveBeginPlay`)

(event `self.ReceiveActorBeginOverlap`
  (params (OtherActor :type "Actor Object Reference"))
  (`GameplayStatics.SpawnSoundAttached` "/Game/Assets/Sounds/Slingshot_Cue.Slingshot_Cue" (`self.StaticMesh`) "None" (0.0 0.0 0.0) (struct) "KeepRelativeOffset" false 1.0 1.0 0.0 null null)
  (bind _asbp_ball (cast `/Game/Blueprints/bp_ball` OtherActor))
  (bind _aspinball_game_mode (cast `/Game/Blueprints/PinballGameMode` (`GameplayStatics.GetGameMode`))
    (:`then`
      (`/Game/Blueprints/PinballGameMode.AddScore` _aspinball_game_mode 20.0))
    (:`CastFailed`
      _))
  (`PrimitiveComponent.AddImpulse` (`/Game/Blueprints/bp_ball.Ball` _asbp_ball) (* (`SceneComponent.GetForwardVector` (`self.Capsule`)) -2500.0) "None" true)
  (bind (_direction _bounce) (`Timeline|SlingBounce` :!via `PlayFromStart`)
    (:`Update`
      (`MeshComponent.SetScalarParameterValueOnMaterials` (`self.StaticMesh`) "PercentOut" _bounce))))

(fn `UserConstructionScript`
  (`PrimitiveComponent.CreateDynamicMaterialInstance` (`self.StaticMesh`) 2 "/Game/Assets/M_MorphBand.M_MorphBand" "None"))