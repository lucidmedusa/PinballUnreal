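; Pinball flipper actor, configurable as left or right through FlipType, that swings up and back with sound.
; The construction script picks mirrored start and end rotations by side, applies the start pose and negates X scale for the right variant.
; Flip and Flop events use MoveComponentTo to rotate between those poses over FlipTime.
; Flip also spawns attached flipper sound cues.
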(event `self.ReceiveBeginPlay`)

(event `Flip`
  (`KismetSystemLibrary.MoveComponentTo` (`self.Flipper`) (0.0 0.0 0.0) (`self.EndRotation`) false false (`self.FlipTime`))
  (`GameplayStatics.SpawnSoundAttached` "/Game/Assets/Sounds/Pinball_FlipperLeft_Cue.Pinball_FlipperLeft_Cue" (`self.Flipper`) "None" (0.0 0.0 0.0) (struct) "KeepRelativeOffset" false 1.0 1.0 0.0 null null)
  (switch `/Game/Blueprints/FlipType` (`self.FlipType`)
    (:`NewEnumerator1`
      (`GameplayStatics.SpawnSoundAttached` "/Game/Assets/Sounds/Pinball_FlipperRight_Cue.Pinball_FlipperRight_Cue" (`self.Flipper`) "None" (0.0 0.0 0.0) (struct) "KeepRelativeOffset" false 1.0 1.0 0.0 null null))))

(event `Flop`
  (`KismetSystemLibrary.MoveComponentTo` (`self.Flipper`) (0.0 0.0 0.0) (`self.StartRotation`) false false (`self.FlipTime`)))

(fn `UserConstructionScript`
  (set `self.StartRotation` (select `/Game/Blueprints/FlipType` (`self.FlipType`) :`NewEnumerator0` (struct :`Yaw` 20.0) :`NewEnumerator1` (struct :`Yaw` -20.0) :!type "Rotator Structure"))
  (set `self.EndRotation` (select `/Game/Blueprints/FlipType` (`self.FlipType`) :`NewEnumerator0` (struct :`Yaw` -20.0) :`NewEnumerator1` (struct :`Yaw` 20.0) :!type "Rotator Structure"))
  (`SceneComponent.K2_SetRelativeRotation` (`self.Flipper`) (`self.StartRotation`) false false)
  (switch `/Game/Blueprints/FlipType` (`self.FlipType`)
    (:`NewEnumerator1`
      (`SceneComponent.SetRelativeScale3D` (`self.Flipper`) (-1.0 1.0 1.0)))))